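; BP_CharacterDialogue is an NPC dialogue component that selects and shows quest, reminder or default lines in a speech bubble.
; Without a DialogueSet it shows default text; otherwise QuestCompleted switches it from objective reminders to stepping through quest lines.
; Each step spawns a WB_Options widget with paired continue/skip responses.
; After the last line it removes the widget, adds the set's end quest, shows closing text and disables talking to the NPC.
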(event `Quest Completed`
  ;[1 1 1] Helper functions
  (set `self.CurrentDialog` -1)
  (set `self.DialogInProgress` true))

(event `Set Speech Bubble`
  (params (SpeechBubble :type "/Game/_MissionDesign/_Base/NPC/WB_SpeechBubble Object Reference") (NPC :type "/Game/_MissionDesign/_Base/NPC/BP_NPC Object Reference"))
  ;[1 1 1] Helper functions
  (set `self.Speech Bubble` SpeechBubble)
  (set `self.NPC` NPC))

(event `Cont Dialogue`
  ;[1 1 1] Dialogue "Tree" - Checks npc status to choose what dialogue to play when interacted with
  (if (`KismetSystemLibrary.IsValid` (stale `Dialogue` _output_get)) :!label _label
    (if (`self.DialogInProgress`)
      (`self.Start Quest Dialogue`)
      (else
        (`self.Default Quest Dialogue`)))
    (else
      (`self.Default Dialogue` (stale `Dialogue` `Default Dialogue`)))))

(event `Dialogue`
  (params (DialogueSet :type "/Game/_MissionDesign/_Base/NPC/Dialogue_DA/PDA_DialogueSet Object Reference") (`Default Dialogue` :type String))
  ;[1 1 1] Dialogue "Tree" - Checks npc status to choose what dialogue to play when interacted with
  (bind _output_get (set `self.Dialogue Set` DialogueSet))
  (goto _label))

(event `Start Quest Dialogue`
  (bind _currentdialog (`self.CurrentDialog`))
  (bind _options_widget (`self.Options Widget`))
  (bind _options_widget_2 (`self.Options Widget`))
  (bind _dialogue_set (`self.Dialogue Set`))
  (bind _responses (`/Game/_MissionDesign/_Base/NPC/Dialogue_DA/PDA_DialogueSet.Responses` _dialogue_set))
  (bind _quest_dialogue (`/Game/_MissionDesign/_Base/NPC/Dialogue_DA/PDA_DialogueSet.Quest Dialogue` _dialogue_set))
  ;[1 1 1] Quest Dialogue - Goes through npc quest dialogue and allows player to give responses
  (`/Engine/EditorBlueprintResources/StandardMacros.IsValid` _options_widget_2
    (:`Is Valid`
      (`Widget.RemoveFromParent` _options_widget_2)
      (`KismetSystemLibrary.CollectGarbage`))
    (:`Is Not Valid`
      _))
  (`/Engine/EditorBlueprintResources/StandardMacros.IncrementInt` (`self.CurrentDialog`)
    (:`  `
      (bind _returnvalue (`|CreateWidget` "/Game/_MissionDesign/_Base/NPC/WB_Options.WB_Options_C" (`GameplayStatics.GetPlayerController` 0) (`|GetArrayItem` _responses (* (`self.CurrentDialog`) 2)) (`|GetArrayItem` _responses (+ (* (`self.CurrentDialog`) 2) 1)) self))
      (bind _output_get (set `self.Options Widget` _returnvalue))
      (`UserWidget.AddToViewport` _output_get 0)
      (if (<= _currentdialog (- (`KismetArrayLibrary.Array_Length` _quest_dialogue) 1))
        (`/Game/_MissionDesign/_Base/NPC/WB_SpeechBubble.SetText` (`self.Speech Bubble`) (`|GetArrayItem` _quest_dialogue _currentdialog))
        (else
          (set `self.DialogInProgress` false)
          (`/Engine/EditorBlueprintResources/StandardMacros.IsValid` _options_widget
            (:`Is Valid`
              (`Widget.RemoveFromParent` _options_widget)
              (`KismetSystemLibrary.CollectGarbage`))
            (:`Is Not Valid`
              _))
          (`self.End Quest Dialogue`))))))

(event `End Quest Dialogue`
  ;[1 1 1] One time dialogue to mark the end of the npc's quest dialogue
  (`/Game/_MissionDesign/_Base/QuestSystem/BFL_QuestSystem.AddQuest` (`/Game/_MissionDesign/_Base/NPC/Dialogue_DA/PDA_DialogueSet.EndQuest` (`self.Dialogue Set`)))
  (`/Game/_MissionDesign/_Base/NPC/WB_SpeechBubble.SetText` (`self.Speech Bubble`) (`/Game/_MissionDesign/_Base/NPC/Dialogue_DA/PDA_DialogueSet.End Quest Dialogue` (`self.Dialogue Set`)))
  (set `/Game/_MissionDesign/_Base/NPC/BP_NPC.CanBeSpokenTo` false (`self.NPC`)))

(event `Default Quest Dialogue`
  ;[1 1 1] reminds player their objective
  (`/Game/_MissionDesign/_Base/NPC/WB_SpeechBubble.SetText` (`self.Speech Bubble`) (`/Game/_MissionDesign/_Base/NPC/Dialogue_DA/PDA_DialogueSet.Default Quest Dialogue` (`self.Dialogue Set`))))

(event `Default Dialogue`
  (params (Dialogue :type String))
  ;[1 1 1] If NPC is not part of current quest, play default dialogue
  (`/Game/_MissionDesign/_Base/NPC/WB_SpeechBubble.SetText` (`self.Speech Bubble`) Dialogue))