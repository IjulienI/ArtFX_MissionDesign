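; Base NPC Blueprint that lets the player talk to it with E while inside its sphere trigger.
; Speaking shows a speech bubble widget, feeds the dialogue component the set mapped to the current quest tag plus a default, and increments that quest's speak action.
; Leaving range hides the bubble, resets running dialogue and removes the options widget.
; Input is polled on Tick; the bubble-to-camera rotation is disconnected.
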(event `self.ReceiveBeginPlay`
  ;[1 1 1] gain access to speechbubble custom events
  (bind _aswb_speech_bubble (cast `/Game/_MissionDesign/_Base/NPC/WB_SpeechBubble` (`WidgetComponent.GetWidget` (`self.Widget`))))
  (`/Game/_MissionDesign/_Base/NPC/BP_CharacterDialogue.Set Speech Bubble` (`self.BP_CharacterDialogue`) _aswb_speech_bubble self))

(event `self.ReceiveTick`
  (params (DeltaSeconds :type "Float (single-precision)"))
  ;[1 1 1] Rotate speech bubble to player and !! Check input
  ;;[1 0 0] should be player input
  (if (`PlayerController.WasInputKeyJustPressed` (`GameplayStatics.GetPlayerController` 0) "E")
    (`self.Speak`)))

(event `Speak`
  ;[1 1 1] Checks if npc can speak to player, then checks quest game tag to set current dialogue
  (if (`self.CanBeSpokenTo`)
    (`SceneComponent.SetHiddenInGame` (`self.Widget`) false false)
    (bind _questdialogues (`self.CheckActiveQuest` (`/Game/_MissionDesign/_Base/QuestSystem/BFL_QuestSystem.GetCurrentQuest`)))
    (`/Game/_MissionDesign/_Base/NPC/BP_CharacterDialogue.Dialogue` (`self.BP_CharacterDialogue`) _questdialogues (`self.DefaultDialogue`))
    (`/Game/_MissionDesign/_Base/QuestSystem/BFL_QuestSystem.IncrementAction` (`/Game/_MissionDesign/_Base/QuestSystem/BFL_QuestSystem.GetCurrentQuest`) (`self.SpeakTag`))))

(event `self.Sphere.OnComponentBeginOverlap`
  (params (OverlappedComponent :type "PrimitiveComponent Object Reference") (OtherActor :type "Actor Object Reference") (OtherComp :type "PrimitiveComponent Object Reference") (OtherBodyIndex :type Integer) (bFromSweep :type Boolean) (SweepResult :type "HitResult Structure (by ref)"))
  ;[1 1 1] If player in range, allow npc to react to interaction input
  (if (== OtherActor (`GameplayStatics.GetPlayerCharacter` 0))
    (set `self.CanBeSpokenTo` true)))

(event `self.Sphere.OnComponentEndOverlap`
  (params (OverlappedComponent :type "PrimitiveComponent Object Reference") (OtherActor :type "Actor Object Reference") (OtherComp :type "PrimitiveComponent Object Reference") (OtherBodyIndex :type Integer))
  (bind _bp_characterdialogue (`self.BP_CharacterDialogue`))
  (bind _options_widget (`/Game/_MissionDesign/_Base/NPC/BP_CharacterDialogue.Options Widget` (`self.BP_CharacterDialogue`)))
  ;[1 1 1] If player leaves range
  (if (== OtherActor (`GameplayStatics.GetPlayerCharacter` 0))
    (`|ExecutionSequence`
      (:`then_0`
        (`SceneComponent.SetHiddenInGame` (`self.Widget`) true false)
        (set `self.CanBeSpokenTo` false))
      (:`then_1`
        (if (`/Game/_MissionDesign/_Base/NPC/BP_CharacterDialogue.DialogInProgress` _bp_characterdialogue)
          (set `/Game/_MissionDesign/_Base/NPC/BP_CharacterDialogue.CurrentDialog` -1 _bp_characterdialogue)))
      (:`then_2`
        (`/Engine/EditorBlueprintResources/StandardMacros.IsValid` _options_widget
          (:`Is Valid`
            (`Widget.RemoveFromParent` _options_widget)
            (`KismetSystemLibrary.CollectGarbage`)))))))

(fn `CheckActiveQuest`
  (params (`Active Quest` :type "GameplayTag Structure"))
  (returns (QuestDialogues :type "/Game/_MissionDesign/_Base/NPC/Dialogue_DA/PDA_DialogueSet Object Reference"))
  (return (`BlueprintMapLibrary.Map_Find` (`self.Dialogues`) `Active Quest`)))

(fn `UserConstructionScript`)