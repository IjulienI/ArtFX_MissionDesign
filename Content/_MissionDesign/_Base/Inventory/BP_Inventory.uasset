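; BP_Inventory stores the player's items as a map from item tag to thumbnail texture and keeps the HUD inventory display in step with it.
; AddItem inserts an entry, then adds an item box to the InventoryWidget on the first player controller's HUD_Base.
; UseItem checks for the tag, removes the entry and its item box when present, and returns whether the item was found.
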(event `Add Item`
  (params (Item :type Name) (Texture :type "Texture Object Reference"))
  (`BlueprintMapLibrary.Map_Add` (`self.Items`) Item Texture)
  (bind _ashud_base (cast `/Game/_MissionDesign/_Base/_Common/_Managers/HUD_Base` (`PlayerController.GetHUD` (`GameplayStatics.GetPlayerController` 0))))
  (`/Game/_MissionDesign/_Base/_Common/_Managers/WB_Inventory.Add Item Box` (`/Game/_MissionDesign/_Base/_Common/_Managers/HUD_Base.InventoryWidget` _ashud_base) Item Texture))

(fn `Use Item`
  (params (`Item Tag` :type Name))
  (returns (`Can Use` :type Boolean))
  (bind _items (`self.Items`))
  (bind _keys (`BlueprintMapLibrary.Map_Keys` _items))
  (if (`KismetArrayLibrary.Array_Contains` _keys `Item Tag`)
    (`BlueprintMapLibrary.Map_Remove` _items (`local.Item Tag`))
    (bind _ashud_base (cast `/Game/_MissionDesign/_Base/_Common/_Managers/HUD_Base` (`PlayerController.GetHUD` (`GameplayStatics.GetPlayerController` 0))))
    (`/Game/_MissionDesign/_Base/_Common/_Managers/WB_Inventory.Remove Item Box` (`/Game/_MissionDesign/_Base/_Common/_Managers/HUD_Base.InventoryWidget` _ashud_base) (`local.Item Tag`))
    (return true)
    (else
      (return false))))