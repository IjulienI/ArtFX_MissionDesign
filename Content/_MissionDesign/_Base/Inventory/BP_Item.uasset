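; BP_Item is a pickup actor that adds itself to the player's inventory when touched.
; On sphere overlap by the player character, it passes its ItemTag and Thumbnail to the player's BP_Inventory component, then destroys itself a tick later.
; The construction script inserts ItemTag into the actor's Tags at index 1.
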(event `self.Sphere.OnComponentBeginOverlap`
  (params (OverlappedComponent :type "PrimitiveComponent Object Reference") (OtherActor :type "Actor Object Reference") (OtherComp :type "PrimitiveComponent Object Reference") (OtherBodyIndex :type Integer) (bFromSweep :type Boolean) (SweepResult :type "HitResult Structure (by ref)"))
  (bind _returnvalue (`GameplayStatics.GetPlayerCharacter` 0))
  (if (== OtherActor _returnvalue)
    (`/Game/_MissionDesign/_Base/Inventory/BP_Inventory.Add Item` (`self.GetComponentByClass` _returnvalue "/Game/_MissionDesign/_Base/Inventory/BP_Inventory.BP_Inventory_C") (`self.Item Tag`) (`self.Thumbnail`))
    (`KismetSystemLibrary.DelayUntilNextTick`)
    (`self.K2_DestroyActor`)))

(fn `UserConstructionScript`
  (`KismetArrayLibrary.Array_Insert` (`self.Tags`) (`self.Item Tag`) 1))