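; Quest system component that registers quests and builds a storage entry for each.
; AddQuest appends the quest to Quests, then FormatStorage stores it in QuestStorage alongside FormatedActions and FormatedNeededObjects.
; FormatStorage adds action and needed-object keys only to Keys() copies, so it never fills those maps.
; QuestFinish and IncrementAction are unimplemented stubs, and the event graph is empty.
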(fn `AddQuest`
  (params (NewQuest :type "/Game/_MissionDesign/_Base/QuestSystem/BDA_BaseQuest Object Reference (by ref)"))
  (`KismetArrayLibrary.Array_Add` (`self.Quests`) NewQuest)
  (`self.FormatStorage` (`local.NewQuest`))
  (return))

(fn `FormatStorage`
  (params (Quest :type "/Game/_MissionDesign/_Base/QuestSystem/BDA_BaseQuest Object Reference"))
  (locals (FormatedActions :type "Map of GameplayTag Structure to Integer") (FormatedNeededObjects :type "Map of Actor Class Reference to Integer"))
  (bind _keys (`BlueprintMapLibrary.Map_Keys` (`/Game/_MissionDesign/_Base/QuestSystem/BDA_BaseQuest.Action` (`local.Quest`))))
  (for _array_element _keys
    (bind _keys_2 (`BlueprintMapLibrary.Map_Keys` (`local.FormatedActions`)))
    (`KismetArrayLibrary.Array_Add` _keys_2 _array_element))
  (bind _keys_3 (`BlueprintMapLibrary.Map_Keys` (`/Game/_MissionDesign/_Base/QuestSystem/BDA_BaseQuest.NeededObjects` (`local.Quest`))))
  (for _array_element_2 _keys_3
    (bind _keys_4 (`BlueprintMapLibrary.Map_Keys` (`local.FormatedNeededObjects`)))
    (`KismetArrayLibrary.Array_Add` _keys_4 _array_element_2))
  (`KismetArrayLibrary.Array_Add` (`self.QuestStorage`) (make `/Game/_MissionDesign/_Base/QuestSystem/STRUCT_QuestStorage` (`local.Quest`) (`local.FormatedActions`) (`local.FormatedNeededObjects`)))
  (return))

(fn `IncrementAction`
  (params (Tag :type "GameplayTag Structure") (Quest :type "/Game/_MissionDesign/_Base/QuestSystem/BDA_BaseQuest Object Reference (by ref)")))

(fn `QuestFinish`
  (params (Quest :type "/Game/_MissionDesign/_Base/QuestSystem/BDA_BaseQuest Object Reference")))